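; Gameplay ability for the Rock augmentation skill that launches BP_Rock projectiles using velocity impulses.
; On activation it commits, then applies GE_CoolDown with a set-by-caller magnitude.
; Ability level selects one straight rock, a three-rock spread, or two spreads separated by a short delay, with EndAbility called after each straight throw.
; ThrowRock spawns and aims from player pawn 0, rotated by a yaw offset; the RPC events are empty.
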(event `RPC_Server`)

(event `RPC_Client`)

(event `self.K2_ActivateAbility`
  (`self.K2_CommitAbility`)
  (bind _returnvalue (`AbilitySystemBlueprintLibrary.AssignTagSetByCallerMagnitude` (`self.MakeOutgoingGameplayEffectSpec` "/Game/Blueprints/Skill/GE_CoolDown.GE_CoolDown_C") (struct :`TagName` "Ability.Augmentation.Rock") (`self.CDT`)))
  (`self.K2_ApplyGameplayEffectSpecToOwner` _returnvalue)
  (switch `int` (`self.GetAbilityLevel`)
    (:`0`
      (`self.Throw Rock` 0.0 :!label _label)
      (`self.K2_EndAbility`))
    (:`1`
      (goto _label))
    (:`2`
      (`|ExecutionSequence` :!label _label_2
        (:`then_0`
          (goto _label))
        (:`then_1`
          (`self.Throw Rock` 15.0)
          (`self.Throw Rock` -15.0))))
    (:`3`
      (`|ExecutionSequence`
        (:`then_0`
          (goto _label_2))
        (:`then_1`
          (`KismetSystemLibrary.Delay` 0.1)
          (goto _label_2))))))

(fn `Throw Rock`
  (params (direction :type "Float (double-precision)"))
  (bind _returnvalue (`GameplayStatics.GetPlayerPawn` 0))
  (bind _returnvalue_2 (`|SpawnActorFromClass` "/Game/Blueprints/Skill/BP_Rock.BP_Rock_C" (`KismetMathLibrary.MakeTransform` (+ (`Actor.K2_GetActorLocation` _returnvalue) (0.0 0.0 0.0) (`KismetMathLibrary.GreaterGreater_VectorRotator` (* (`Actor.GetActorForwardVector` _returnvalue) (50.0 50.0 50.0)) (`KismetMathLibrary.MakeRotator` 0.0 0.0 direction))) (`Pawn.GetControlRotation` _returnvalue)) "Undefined" "MultiplyWithRoot" null null))
  (`PrimitiveComponent.AddImpulse` (`/Game/Blueprints/Skill/BP_Rock.Rock_0` _returnvalue_2) (* (`KismetMathLibrary.GreaterGreater_VectorRotator` (`SceneComponent.GetForwardVector` (`Actor.RootComponent` _returnvalue)) (`KismetMathLibrary.MakeRotator` 0.0 0.0 direction)) (2000.0 2000.0 2000.0)) "None" true))