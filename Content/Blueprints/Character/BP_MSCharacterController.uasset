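; Player controller for BP_MSCharacter that handles Enhanced Input movement and right-mouse aiming.
; On BeginPlay the local controller adds the movement mapping context and caches the character, whose Death flag gates all input through a macro.
; Holding right mouse sets Aiming and yaws the pawn by the mouse's angle from screen center, using dot and cross products.
; Rotation applies locally and through a Server_SetActorRotation event.
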(event `self.ReceiveBeginPlay`
  (if (`self.IsLocalPlayerController`)
    (`EnhancedInputSubsystemInterface.AddMappingContext` (subsystem `EnhancedInputLocalPlayerSubsystem`) "/Game/Blueprints/Character/Input/IMC_MSMovingControl.IMC_MSMovingControl" 0 (struct))
    (bind _asbp_mscharacter (cast `/Game/Blueprints/Character/BP_MSCharacter` (`self.K2_GetPawn`)))
    (set `self.BP MSCharacter` _asbp_mscharacter)))

(event `EnhancedInput|/Game/Blueprints/Character/Input/IA_MSMove`
  (params (ActionValue :type "Vector2D Structure") (ElapsedSeconds :type "Float (double-precision)") (TriggeredSeconds :type "Float (double-precision)") (InputAction :type "InputAction Object Reference" :default "/Game/Blueprints/Character/Input/IA_MSMove.IA_MSMove"))
  (bind (_returnvalue_roll _returnvalue_pitch _returnvalue_yaw) (`KismetMathLibrary.BreakRotator` (`self.GetControlRotation`)))
  (bind _returnvalue (`self.K2_GetPawn`))
  (:`Triggered`
    (`self.IsPlayerDeath?`
      (:`Alive`
        (`Pawn.AddMovementInput` _returnvalue (`KismetMathLibrary.GetRightVector` (`KismetMathLibrary.MakeRotator` 0.0 0.0 _returnvalue_yaw)) ActionValue_X false)
        (`Pawn.AddMovementInput` _returnvalue (`KismetMathLibrary.GetForwardVector` (`KismetMathLibrary.MakeRotator` 0.0 0.0 _returnvalue_yaw)) ActionValue_Y false)))))

(event `EnhancedInput|/Game/Blueprints/Character/Input/IA_MSMouseRightBtn`
  (params (ActionValue :type Boolean) (ElapsedSeconds :type "Float (double-precision)") (TriggeredSeconds :type "Float (double-precision)") (InputAction :type "InputAction Object Reference" :default "/Game/Blueprints/Character/Input/IA_MSMouseRightBtn.IA_MSMouseRightBtn"))
  (:`Triggered`
    (`self.IsPlayerDeath?`
      (:`Alive`
        (`self.SetPlayerRotationToMouse` (`GameplayStatics.GetPlayerController` 0)))))
  (:`Started`
    (`self.IsPlayerDeath?`
      (:`Alive`
        (set `self.Aiming` true))))
  (:`Completed`
    (`self.IsPlayerDeath?`
      (:`Alive`
        (set `self.Aiming` false)))))

(event `Server_SetActorRotation`
  (params (Target :type "Actor Object Reference") (`New Rotation Z (Yaw)` :type "Float (single-precision)"))
  (`self.K2_SetActorRotation` Target (`KismetMathLibrary.MakeRotator` 0.0 0.0 `New Rotation Z (Yaw)`) false))

(fn `SetPlayerRotationToMouse`
  (params (PlayerController :type "PlayerController Object Reference"))
  (locals (MouseVector :type "Vector2D Structure") (UpVector :type "Vector2D Structure"))
  (bind _returnvalue (`self.K2_GetPawn`))
  (bind _returnvalue_2 (`self.K2_GetPawn`))
  (bind (_locationx _locationy) (`self.GetMousePosition` PlayerController))
  (bind _characterdegree (`self.CharacterDegree`))
  (bind _output_get (set `local.MouseVector` (- (`KismetMathLibrary.MakeVector2D` _locationx _locationy) (/ (`WidgetLayoutLibrary.GetViewportSize`) (2.0 2.0)))))
  (bind _output_get_2 (set `local.UpVector` (0.0 -1.0)))
  (bind _returnvalue_3 (`KismetMathLibrary.Normal2D` _output_get))
  (bind _returnvalue_4 (`KismetMathLibrary.Normal2D` _output_get_2))
  (set `self.CharacterDegree` (`KismetMathLibrary.DegAcos` (`KismetMathLibrary.DotProduct2D` _returnvalue_3 _returnvalue_4)))
  (if (< (`KismetMathLibrary.CrossProduct2D` _returnvalue_3 _returnvalue_4) 0.0)
    (`self.K2_SetActorRotation` _returnvalue_2 (`KismetMathLibrary.MakeRotator` 0.0 0.0 _characterdegree) false)
    (`self.Server_SetActorRotation` _returnvalue_2 _characterdegree)
    (else
      (bind _output_get_3 (set `self.CharacterDegree` (* (`self.CharacterDegree`) -1.0)))
      (`self.K2_SetActorRotation` _returnvalue (`KismetMathLibrary.MakeRotator` 0.0 0.0 _output_get_3) false)
      (`self.Server_SetActorRotation` _returnvalue _output_get_3))))

(fn `UserConstructionScript`)