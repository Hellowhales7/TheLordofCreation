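; Networked player character built on GAS, handling health, experience, leveling, death, revival and HUD widgets.
; Gameplay effects change attributes, and derived percentages drive RepNotify chains into death or level-up, with SpawnRange overlap reviving the dead.
; Level-up opens the augmentation UI and a two-player ready count that toggles game pause.
; Selected abilities gain levels on repeat picks, and the server re-grants and activates them every Tick while copying controller aim state.
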(event `Server_ApplyInitalGameplayEffect`
  (`self.Multicast_InitialGameplayEffect`))

(event `Apply Invincible`
  (set `self.bInvincible` true)
  (`KismetSystemLibrary.K2_SetTimer` null "EndInvincible" (`self.InvincibleTime`)))

(event `Multicast_InitialGameplayEffect`
  (`AbilitySystemComponent.BP_ApplyGameplayEffectToSelf` :`self` (`self.AbilitySystemComponent`) :`GameplayEffectClass` "/Game/Blueprints/GAS/GE/GE_InitalizeAttributes.GE_InitalizeAttributes_C"))

(event `ApplyAddHealthEffect`
  ;[1 1 1] Debug
  (`/Engine/EditorBlueprintResources/ActorMacros.Switch Has Authority`
    (:`Authority`
      (`AbilitySystemComponent.BP_ApplyGameplayEffectToSelf` :`self` (`self.AbilitySystemComponent`) :`GameplayEffectClass` "/Game/Blueprints/GAS/GE/GE_AddHealth.GE_AddHealth_C"))
    (:`Remote`
      (`self.Server_AddHealthEffect`))))

(event `Key|F`
  (params (Key :type "Key Structure"))
  ;[1 1 1] Debug
  (:`Pressed`
    (`self.ApplyAddHealthEffect`)
    (`self.SetHealthPercent`)
    (`KismetSystemLibrary.PrintString` (`KismetStringLibrary.Conv_BoolToString` (`self.Death`)))))

(event `self.ReceiveBeginPlay`
  (bind _asbp_mscharacter_controller (cast `/Game/Blueprints/Character/BP_MSCharacterController` (`self.GetController`)))
  (set `self.BP MSCharacter Controller` _asbp_mscharacter_controller)
  (`self.AddWidget`)
  (`self.Server_ApplyInitalGameplayEffect`)
  (set `PlayerController.bShowMouseCursor` true (`self.BP MSCharacter Controller`))
  (`KismetSystemLibrary.Delay` 0.25)
  (`self.SetHealthPercent`)
  (`self.SetExpPercent`))

(event `Server_AddHealthEffect`
  ;[1 1 1] Debug
  (`AbilitySystemComponent.BP_ApplyGameplayEffectToSelf` :`self` (`self.AbilitySystemComponent`) :`GameplayEffectClass` "/Game/Blueprints/GAS/GE/GE_AddHealth.GE_AddHealth_C"))

(event `self.ReceiveTick`
  (params (DeltaSeconds :type "Float (single-precision)"))
  (`/Engine/EditorBlueprintResources/ActorMacros.Switch Has Authority`
    (:`Authority`
      (`self.SetSpeedAndShouldMove`)
      ;[1 1 1] controller가 서버에 하나밖에없어서 controller에 구현한거 character로 옮겨야함(is not valid가 클라인데 클라에서 변수 set이 안되서 동기화 불가)
      (bind _bp_mscharacter_controller (`self.BP MSCharacter Controller`)
        (:`then`
          (set `self.Aiming` (`/Game/Blueprints/Character/BP_MSCharacterController.Aiming` _bp_mscharacter_controller))
          (set `self.CharacterDegree` (`/Game/Blueprints/Character/BP_MSCharacterController.CharacterDegree` _bp_mscharacter_controller)))
        (:`else`
          _))
      (`self.ActiveAbility`))))

(event `Key|Five`
  (params (Key :type "Key Structure"))
  ;[1 1 1] Open Option Menu
  (:`Pressed`
    (if (`self.MenuVisible`)
      (`Widget.RemoveFromParent` (`self.Menu`))
      (`Widget.RemoveFromParent` (`self.OptionMenu`))
      (set `self.MenuVisible` false)
      (else
        (set `self.MenuVisible` true)
        (bind _returnvalue (`|CreateWidget` "/Game/Blueprints/Character/CharacterUI/WBP_Menu.WBP_Menu_C"))
        (bind _output_get (set `self.Menu` _returnvalue))
        (`UserWidget.AddToViewport` _output_get 0)))))

(event `Server_ApplyDamage`
  (params (DamagedActor :type "Actor Object Reference") (BaseDamage :type "Float (single-precision)"))
  (bind _attackpower_basevalue (break `GameplayAttributeData` (`PlayerAttributeSet.AttackPower` (`self.PlayerAttributeSet`))))
  ;[1 1 1] Apply Damage
  (`GameplayStatics.ApplyDamage` DamagedActor (+ (+ BaseDamage _attackpower_basevalue) 50.0)))

(event `/Game/Blueprints/BlueprintInterface/BPI_HandleDamage.Damaged`
  (params (DamageAmount :type Integer) (`Overlapped Actor` :type "/Game/Blueprints/Character/BP_MSCharacter Object Reference"))
  (bind _defensivepower_basevalue (break `GameplayAttributeData` (`PlayerAttributeSet.DefensivePower` (`self.PlayerAttributeSet`))))
  ;[1 1 1] Damaged
  (if (== `Overlapped Actor` (`GameplayStatics.GetPlayerCharacter` 0))
    (bind _returnvalue (`|CreateWidget` "/Game/Blueprints/Character/CharacterUI/WBP_OnHitEffect.WBP_OnHitEffect_C"))
    (`UserWidget.AddToViewport` _returnvalue 0))
  (`/Engine/EditorBlueprintResources/ActorMacros.Switch Has Authority`
    (:`Authority`
      (`self.HandleDamage` (* (- DamageAmount _defensivepower_basevalue) -1.0))
      (`self.SetHealthPercent`))))

(event `Key|Tab`
  (params (Key :type "Key Structure"))
  (:`Pressed`
    (bind _returnvalue (`|CreateWidget` "/Game/Blueprints/Character/CharacterUI/WBP_MySkill.WBP_MySkill_C"))
    (bind _output_get (set `self.SkillWBP` _returnvalue))
    (`UserWidget.AddToViewport` _output_get 0))
  (:`Released`
    (`Widget.RemoveFromParent` (`self.SkillWBP`))))

(event `Level Up`
  ;[1 1 1] Level Up
  (`AbilitySystemComponent.BP_ApplyGameplayEffectToSelf` :`self` (`self.AbilitySystemComponent`) :`GameplayEffectClass` "/Game/Blueprints/GAS/GE/GE_LevelUp.GE_LevelUp_C")
  (`self.SetExpPercent`)
  (bind _skillwbp (`self.SkillWBP`)
    (:`then`
      (`Widget.RemoveFromParent` _skillwbp))
    (:`else`
      _))
  (`self.ShowAugmentationUI`))

(event `/Game/Blueprints/BlueprintInterface/BPI_HandleExp.GetExp`
  (params (ExpAmount :type "Float (double-precision)"))
  ;[1 1 1] GetExp
  (bind _returnvalue (`AbilitySystemBlueprintLibrary.AssignTagSetByCallerMagnitude` (`AbilitySystemComponent.MakeOutgoingSpec` :`self` (`self.AbilitySystemComponent`) :`GameplayEffectClass` "/Game/Blueprints/GAS/GE/GE_AddExp.GE_AddExp_C" :`Level` 1.0) (struct :`TagName` "ability") ExpAmount))
  (`AbilitySystemComponent.BP_ApplyGameplayEffectSpecToSelf` (`self.AbilitySystemComponent`) _returnvalue)
  (`self.SetExpPercent`))

(event `Ability Selected`
  (params (Ability :type "/Game/Blueprints/GAS/GA/Augmentation/GA_Base Class Reference"))
  ;[1 1 1] Ability Manage(Temp)
  (set `self.SelectedAbility` Ability)
  (if (`KismetArrayLibrary.Array_Contains` (`self.PlayerAbilities`) (`self.SelectedAbility`))
    (`self.SelectedAbility Upgrade` (`self.SelectedAbility`))
    (else
      (`KismetArrayLibrary.Array_Add` (`self.PlayerAbilities`) (`self.SelectedAbility`))
      (`BlueprintMapLibrary.Map_Add` (`self.AbilitiesLevel`) (`self.SelectedAbility`) 1)
      (for (_ _array_index) (`self.PlayerAbilities`)
        (`KismetArrayLibrary.Array_Set` (`self.AbilityLevels`) _array_index 1 true)))))

(event `PlayerDie`
  (`/Engine/EditorBlueprintResources/ActorMacros.Switch Has Authority`
    (:`Authority`
      (`PrimitiveComponent.SetCollisionEnabled` (`self.CapsuleComponent`) "NoCollision")
      (`PrimitiveComponent.SetCollisionEnabled` (`self.Mesh`) "NoCollision")
      (`PrimitiveComponent.SetCollisionResponseToChannel` (`self.CapsuleComponent`) "ECC_GameTraceChannel4" "ECR_Ignore"))))

(event `SelectedAbility Upgrade`
  (params (SelectedAbility :type "/Game/Blueprints/GAS/GA/Augmentation/GA_Base Class Reference"))
  (bind (_value _returnvalue) (`BlueprintMapLibrary.Map_Find` (`self.AbilitiesLevel`) SelectedAbility))
  ;[1 1 1] Ability Manage(Temp)
  (if _returnvalue
    (`BlueprintMapLibrary.Map_Add` (`self.AbilitiesLevel`) SelectedAbility (+ _value 1))
    (`KismetArrayLibrary.Array_Set` (`self.AbilityLevels`) (`KismetArrayLibrary.Array_Find` (`self.PlayerAbilities`) SelectedAbility) _value true)))

(event `Revive`
  (set `self.Death` false)
  (`AbilitySystemComponent.BP_ApplyGameplayEffectToSelf` :`self` (`self.AbilitySystemComponent`) :`GameplayEffectClass` "/Game/Blueprints/GAS/GE/GE_ReviveHealth.GE_ReviveHealth_C")
  (`self.SetHealthPercent`)
  (`PrimitiveComponent.SetCollisionResponseToChannel` (`self.CapsuleComponent`) "ECC_GameTraceChannel4" "ECR_Overlap")
  (`PrimitiveComponent.SetCollisionEnabled` (`self.CapsuleComponent`) "QueryAndPhysics")
  (`PrimitiveComponent.SetCollisionEnabled` (`self.Mesh`) "QueryAndPhysics"))

(event `PlayerReadyCheck`
  (bind _servercharacter0 (`self.ServerCharacter0`))
  ;[1 1 1] Sync Pause Start/End
  (bind _outactors (`GameplayStatics.GetAllActorsOfClass` "BP_MSCharacter_C"))
  (for _array_element _outactors
    (if (`self.HasAuthority` _array_element)
      (bind _output_get (set `/Game/Blueprints/Character/BP_MSCharacter.ReadyPlayerCount` (+ (`/Game/Blueprints/Character/BP_MSCharacter.ReadyPlayerCount` _array_element) 1) _array_element))
      (set `self.ServerCharacter0` _array_element)))
  (if (== _output_get 2)
    (bind _output_get_2 (set `/Game/Blueprints/Character/BP_MSCharacter.PauseCount` (+ (`/Game/Blueprints/Character/BP_MSCharacter.PauseCount` _servercharacter0) 1) _servercharacter0))
    (if (`self.Is Odd Number` _output_get_2)
      (`GameplayStatics.SetGamePaused` true)
      (else
        (`GameplayStatics.SetGamePaused` false)))
    (set `/Game/Blueprints/Character/BP_MSCharacter.ReadyPlayerCount` 0 (`self.ServerCharacter0`))))

(event `self.SpawnRange.OnComponentBeginOverlap`
  (params (OverlappedComponent :type "PrimitiveComponent Object Reference") (OtherActor :type "Actor Object Reference") (OtherComp :type "PrimitiveComponent Object Reference") (OtherBodyIndex :type Integer) (bFromSweep :type Boolean) (SweepResult :type "HitResult Structure (by ref)"))
  (if (`self.Death`)
    (`self.Revive`)))

(fn `ActiveAbility`
  (bind _abilitysystemcomponent (`self.AbilitySystemComponent`))
  (for _array_element (`self.PlayerAbilities`)
    (bind _returnvalue (`AbilitySystemComponent.K2_GiveAbility` _abilitysystemcomponent _array_element (`BlueprintMapLibrary.Map_Find` (`self.AbilitiesLevel`) _array_element) -1))
    (`AbilitySystemComponent.TryActivateAbility` _abilitysystemcomponent _returnvalue true)))

(fn `AddWidget`
  (bind _returnvalue (`|CreateWidget` "/Game/Blueprints/Character/CharacterUI/WBP_Test.WBP_Test_C" (`self.BP MSCharacter Controller`) self))
  (bind _output_get (set `self.TestHealthBtnUI` _returnvalue))
  (`UserWidget.AddToViewport` _output_get 0)
  (bind _returnvalue_2 (`|CreateWidget` "/Game/Blueprints/Character/CharacterUI/WBP_HealthBar.WBP_HealthBar_C" null self))
  (bind _output_get_2 (set `self.HealthBarUI` _returnvalue_2))
  (`UserWidget.AddToViewport` _output_get_2 0)
  (bind _returnvalue_3 (`|CreateWidget` "/Game/Blueprints/Character/CharacterUI/WBP_ExpBar.WBP_ExpBar_C" null self))
  (bind _output_get_3 (set `self.ExpUI` _returnvalue_3))
  (`UserWidget.AddToViewport` _output_get_3 0))

(fn `EndInvincible`
  (set `self.bInvincible` false))

(fn `GetExpToAllPlayer`
  (bind _outactors (`GameplayStatics.GetAllActorsOfClass` "BP_MSCharacter_C"))
  (for _array_element _outactors
    (`AbilitySystemComponent.BP_ApplyGameplayEffectToSelf` :`self` (`BaseCharacter.AbilitySystemComponent` _array_element) :`GameplayEffectClass` "/Game/Blueprints/GAS/GE/GE_AddExp.GE_AddExp_C")
    (`KismetSystemLibrary.PrintString` "exp")
    (`self.SetExpPercent`)
    (if (>= (`self.ExpPercent`) 1.0)
      (`self.Level Up`))))

(fn `HandleDamage`
  (params (Magnitude :type "Float (single-precision)"))
  (bind _returnvalue (`AbilitySystemBlueprintLibrary.AssignTagSetByCallerMagnitude` (`AbilitySystemComponent.MakeOutgoingSpec` :`self` (`self.AbilitySystemComponent`) :`GameplayEffectClass` "/Game/Blueprints/GAS/GE/GE_Damage.GE_Damage_C" :`Level` 1.0) (struct :`TagName` "ability") Magnitude))
  (`AbilitySystemComponent.BP_ApplyGameplayEffectSpecToSelf` (`self.AbilitySystemComponent`) _returnvalue))

(fn `Is Odd Number`
  (params (Count :type Integer))
  (returns (`Odd Number` :type Boolean))
  (return (== (mod Count 2) 1)))

(fn `OnRep_Death`
  (`self.PlayerDie`))

(fn `OnRep_ExpPercent`
  (if (>= (`self.ExpPercent`) 1.0)
    (set `self.Level` (+ (`self.Level`) 1.0))))

(fn `OnRep_HealthPercent`
  (if (<= (`self.HealthPercent`) 0.0)
    (set `self.Death` true)))

(fn `OnRep_Level`
  (`self.Level Up`))

(fn `SetExpPercent`
  (bind _playerattributeset (`self.PlayerAttributeSet`))
  (bind (_maxexperience_basevalue _maxexperience_currentvalue) (break `GameplayAttributeData` (`PlayerAttributeSet.MaxExperience` _playerattributeset)))
  (bind (_experience_basevalue _experience_currentvalue) (break `GameplayAttributeData` (`PlayerAttributeSet.Experience` _playerattributeset)))
  (set `self.ExpPercent` (/ _experience_currentvalue _maxexperience_currentvalue)))

(fn `SetHealthPercent`
  (bind _playerattributeset (`self.PlayerAttributeSet`))
  (bind (_health_basevalue _health_currentvalue) (break `GameplayAttributeData` (`PlayerAttributeSet.Health` _playerattributeset)))
  (bind (_maxhealth_basevalue _maxhealth_currentvalue) (break `GameplayAttributeData` (`PlayerAttributeSet.MaxHealth` _playerattributeset)))
  (set `self.HealthPercent` (/ _health_currentvalue _maxhealth_currentvalue)))

(fn `SetSpeedAndShouldMove`
  (set `self.Speed` (`KismetMathLibrary.VSizeXY` (`MovementComponent.Velocity` (`self.CharacterMovement`))))
  (set `self.ShouldMove` (and (> (`self.Speed`) 3.0) (!= (`CharacterMovementComponent.GetCurrentAcceleration` (`self.CharacterMovement`)) (0.0 0.0 0.0)))))

(fn `ShowAugmentationUI`
  (bind _bp_mscharacter_controller (`self.BP MSCharacter Controller`)
    (:`then`
      (set `PlayerController.bShowMouseCursor` true _bp_mscharacter_controller)
      (bind _returnvalue (`|CreateWidget` "/Game/Blueprints/Character/CharacterUI/WBP_Augmentation.WBP_Augmentation_C"))
      (`UserWidget.AddToViewport` _returnvalue 0)
      (`self.PlayerReadyCheck`))
    (:`else`)))

(fn `UserConstructionScript`)