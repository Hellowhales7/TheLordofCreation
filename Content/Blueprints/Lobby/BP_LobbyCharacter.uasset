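; Lobby character that displays a player's lobby info through a widget component.
; UpdatePlayerLobbyInfo sets the RepNotify variable PlayerLobbyInfo, whose OnRep passes it to the WBP_PlayerInfo widget and makes the component visible.
; If the widget is not valid yet, the OnRep retries itself on a short timer.
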(event `self.ReceiveBeginPlay`)

(fn `OnRep_PlayerLobbyInfo`
  (bind _returnvalue (`WidgetComponent.GetWidget` (`self.LobbyInfo`)))
  (`/Engine/EditorBlueprintResources/StandardMacros.IsValid` _returnvalue
    (:`Is Valid`
      (bind _aswbp_player_info (cast `/Game/Blueprints/Lobby/LobbyUI/WBP_PlayerInfo` _returnvalue))
      (`/Game/Blueprints/Lobby/LobbyUI/WBP_PlayerInfo.Update` _aswbp_player_info (`self.PlayerLobbyInfo`))
      (`SceneComponent.SetVisibility` (`self.LobbyInfo`) true false))
    (:`Is Not Valid`
      (`KismetSystemLibrary.K2_SetTimer` null "OnRep_PlayerLobbyInfo" 0.1))))

(fn `UpdatePlayerLobbyInfo`
  (params (PlayerLobbyInfo :type "/Game/Blueprints/Lobby/LobbyPlayerInfo Structure"))
  (set `self.PlayerLobbyInfo` PlayerLobbyInfo))

(fn `UserConstructionScript`)