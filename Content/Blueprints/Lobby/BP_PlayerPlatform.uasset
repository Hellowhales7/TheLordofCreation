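; BP_PlayerPlatform is a lobby platform that displays a character for an assigned lobby player controller.
; SpawnCharacter stores the controller, destroys any existing character and spawns a BP_LobbyCharacter at the SpawnTransform component's world transform.
; Clear releases the controller reference and destroys the current character, leaving the platform empty.
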(event `SpawnCharacter`
  (params (LobbyPC :type "PlayerController Object Reference"))
  (set `self.LobbyPC` LobbyPC)
  (bind _currentcharacter (`self.CurrentCharacter`)
    (:`then`
      (`self.K2_DestroyActor` _currentcharacter))
    (:`else`
      _))
  (bind _returnvalue (`|SpawnActorFromClass` "/Game/Blueprints/Lobby/BP_LobbyCharacter.BP_LobbyCharacter_C" (`SceneComponent.K2_GetComponentToWorld` (`self.SpawnTransform`)) "Undefined" "MultiplyWithRoot" null null))
  (set `self.CurrentCharacter` _returnvalue))

(event `Clear`
  (set `self.LobbyPC` null)
  (bind _currentcharacter (`self.CurrentCharacter`)
    (:`then`
      (`self.K2_DestroyActor` _currentcharacter)
      (set `self.CurrentCharacter` null))
    (:`else`)))

(fn `UserConstructionScript`)