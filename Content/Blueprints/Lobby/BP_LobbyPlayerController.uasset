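; Lobby player controller that manages a player's lobby UI, name and ready status.
; On BeginPlay, the local controller shows the cursor, creates WBP_LobbyUI and submits the player name.
; OnServer events update PlayerLobbyInfoPC and pass the controller to BP_LobbyGameMode, with a separate delayed event for retrying that update.
; OnStartMatch shows the UI's loading screen, and a temporary R-key debug binding toggles ready.
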(event `TryAgainUpdatingLobbyInfo`
  (`KismetSystemLibrary.Delay` 0.1)
  (bind _asbp_lobby_game_mode (cast `/Game/Blueprints/Lobby/BP_LobbyGameMode` (`GameplayStatics.GetGameMode`)))
  (`/Game/Blueprints/Lobby/BP_LobbyGameMode.UpdatePlayerLobbyInfo` _asbp_lobby_game_mode self))

(event `self.ReceiveBeginPlay`
  (`self.SetUp`))

(event `SetPlayerNameOnServer`
  (params (PlayerName :type Text))
  (setmembers `/Game/Blueprints/Lobby/LobbyPlayerInfo` :`StructRef` (`self.PlayerLobbyInfoPC`) :`PlayerName` PlayerName)
  (bind _asbp_lobby_game_mode (cast `/Game/Blueprints/Lobby/BP_LobbyGameMode` (`GameplayStatics.GetGameMode`)))
  (`/Game/Blueprints/Lobby/BP_LobbyGameMode.UpdatePlayerLobbyInfo` _asbp_lobby_game_mode self))

(event `ToggleReadyStatusOnServer`
  (bind _playerlobbyinfopc (`self.PlayerLobbyInfoPC`))
  (setmembers `/Game/Blueprints/Lobby/LobbyPlayerInfo` :`StructRef` _playerlobbyinfopc :`Ready` (not (`.Ready_4_8591BA0D463152670F84009484E7164E` (break `/Game/Blueprints/Lobby/LobbyPlayerInfo` _playerlobbyinfopc))))
  (bind _asbp_lobby_game_mode (cast `/Game/Blueprints/Lobby/BP_LobbyGameMode` (`GameplayStatics.GetGameMode`)))
  (`/Game/Blueprints/Lobby/BP_LobbyGameMode.UpdatePlayerLobbyInfo` _asbp_lobby_game_mode self))

(event `Key|R`
  (params (Key :type "Key Structure"))
  ;[1 1 1] Debug(delete later)
  (:`Pressed`
    (`self.ToggleReadyStatusOnServer`)))

(event `OnStartMatch`
  (`/Game/Blueprints/Lobby/LobbyUI/WBP_LobbyUI.ShowLoadingScreen` (`self.LobbyUI`)))

(fn `SetUp`
  (if (`self.IsLocalPlayerController`)
    (set `self.bShowMouseCursor` true)
    (bind _returnvalue (`|GenericCreateObject` "/Game/Blueprints/Lobby/LobbyUI/WBP_LobbyUI.WBP_LobbyUI_C"))
    (bind _output_get (set `self.LobbyUI` _returnvalue))
    (`UserWidget.AddToViewport` _output_get 0)
    (`self.SetPlayerNameOnServer` (`KismetTextLibrary.Conv_StringToText` (`AdvancedSessionsLibrary.GetPlayerName` self)))))

(fn `UserConstructionScript`)