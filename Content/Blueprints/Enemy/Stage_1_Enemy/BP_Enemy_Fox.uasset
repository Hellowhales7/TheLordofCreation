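; BP_Enemy_Fox is a Stage 1 ranged enemy that sets its own combat attributes and shoots projectiles at players.
; A looping FindNearestPlayer timer runs until a character enters DetectRange, which stops AI movement and starts timed attacks.
; Each attack faces the last character to enter and spawns a BP_FoxProjectile carrying AttackPower.
; The search resumes when the range empties, and death plays an animation before destroying the actor.
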(event `self.ReceiveBeginPlay`
  (`parent.ReceiveBeginPlay`)
  (`self.Server_Init`)
  (`self.SetAttributes` 120.0 120.0 15 1.0 60.0 400.0)
  (`KismetSystemLibrary.K2_SetTimer` null "FindNearestPlayer" 0.5 true))

(event `self.DetectRange.OnComponentBeginOverlap`
  (params (OverlappedComponent :type "PrimitiveComponent Object Reference") (OtherActor :type "Actor Object Reference") (OtherComp :type "PrimitiveComponent Object Reference") (OtherBodyIndex :type Integer) (bFromSweep :type Boolean) (SweepResult :type "HitResult Structure (by ref)"))
  (bind _asbp_mscharacter (cast `/Game/Blueprints/Character/BP_MSCharacter` OtherActor))
  (set `self.BP MSCharacter` _asbp_mscharacter)
  (`KismetSystemLibrary.K2_ClearTimer` null "FindNearestPlayer")
  (bind _bp_enemy_aicontroller (`self.BP Enemy AIController`)
    (:`then`
      (`Controller.StopMovement` _bp_enemy_aicontroller)
      (`self.Ranged Attack`))
    (:`else`)))

(event `self.DetectRange.OnComponentEndOverlap`
  (params (OverlappedComponent :type "PrimitiveComponent Object Reference") (OtherActor :type "Actor Object Reference") (OtherComp :type "PrimitiveComponent Object Reference") (OtherBodyIndex :type Integer))
  (if (== (`KismetArrayLibrary.Array_Length` (`PrimitiveComponent.GetOverlappingActors` (`self.DetectRange`) "/Game/Blueprints/Character/BP_MSCharacter.BP_MSCharacter_C")) 0)
    (`KismetSystemLibrary.K2_ClearTimer` null "DoRangedAttack")
    (`KismetSystemLibrary.K2_SetTimer` null "FindNearestPlayer" 0.5 true)))

(event `Ranged Attack`
  (`KismetSystemLibrary.K2_SetTimer` null "DoRangedAttack" 2.0 true))

(event `self.Die`
  (`parent.Die`)
  (`SkeletalMeshComponent.PlayAnimation` (`self.Mesh`) "/Game/Fab/ForestAnimalsPack/Fox/Animations/ANIM_Fox_Death.ANIM_Fox_Death" false)
  (set `self.Death` true)
  (`KismetSystemLibrary.Delay` 2.5)
  (`self.K2_DestroyActor`))

(fn `DoRangedAttack`
  (locals (TargetLocation :type "Vector Structure") (SelfLocation :type "Vector Structure" :default (0.0 0.0 0.0)))
  (bind _returnvalue (`KismetMathLibrary.FindLookAtRotation` (`local.SelfLocation`) (`local.TargetLocation`)))
  (set `local.SelfLocation` (`self.K2_GetActorLocation`))
  (set `local.TargetLocation` (`self.K2_GetActorLocation` (`self.BP MSCharacter`)))
  (`self.K2_SetActorRotation` _returnvalue)
  (`|SpawnActorFromClass` "/Game/Blueprints/Enemy/Stage_1_Enemy/BP_FoxProjectile.BP_FoxProjectile_C" (`KismetMathLibrary.MakeTransform` (`self.K2_GetActorLocation`) _returnvalue) "Undefined" "MultiplyWithRoot" null (`self.AttackPower`) null))

(fn `UserConstructionScript`
  (`parent.UserConstructionScript`))