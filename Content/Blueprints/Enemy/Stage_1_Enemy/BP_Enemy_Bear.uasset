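; Stage 1 bear enemy Blueprint that builds on a parent enemy class.
; BeginPlay runs the parent logic and ServerInit, sets the bear's combat and movement attributes, and starts a looping timer that calls FindNearestPlayer.
; Death runs the parent logic, plays the bear's death animation, sets the Death flag and destroys the actor after a short delay.
; Two custom events wrap MulticastInit and Initalize.
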(event `CustomEvent`
  (`self.Multicast_Init`))

(event `CustomEvent_1`
  (`self.Initalize`))

(event `self.ReceiveBeginPlay`
  (`parent.ReceiveBeginPlay`)
  (`self.Server_Init`)
  (`self.SetAttributes` 250.0 250.0 40 5.0 100.0 300.0)
  (`KismetSystemLibrary.K2_SetTimer` null "FindNearestPlayer" 0.5 true))

(event `self.Die`
  (`parent.Die`)
  (`SkeletalMeshComponent.PlayAnimation` (`self.Mesh`) "/Game/Fab/ForestAnimalsPack/Bear/Animations/ANIM_Bear_Death4Legs.ANIM_Bear_Death4Legs" false)
  (set `self.Death` true)
  (`KismetSystemLibrary.Delay` 2.0)
  (`self.K2_DestroyActor`))

(fn `UserConstructionScript`
  (`parent.UserConstructionScript`))