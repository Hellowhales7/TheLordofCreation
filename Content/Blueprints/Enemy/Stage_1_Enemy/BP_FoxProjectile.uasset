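; BP_FoxProjectile is a projectile for the Stage 1 fox enemy that damages actors it overlaps.
; On BeginPlay it disables gravity on the Projectile component and launches it with a velocity-change impulse along the actor's forward vector, strongly weighted to horizontal.
; Sphere overlaps send DamagedMessage with AttackPower on authority only, without destroying the projectile.
; A Tick-accumulated timer destroys the actor after a few seconds.
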(event `self.ReceiveBeginPlay`
  (`PrimitiveComponent.SetEnableGravity` (`self.Projectile`) false)
  (`PrimitiveComponent.AddImpulse` (`self.Projectile`) (* (`self.GetActorForwardVector`) (1000.0 1000.0 1.0)) "None" true))

(event `self.ReceiveTick`
  (params (DeltaSeconds :type "Float (single-precision)"))
  (bind _output_get (set `self.timer` (+ DeltaSeconds (`self.timer`))))
  (if (>= _output_get 4.0)
    (`self.K2_DestroyActor`)))

(event `self.Sphere.OnComponentBeginOverlap`
  (params (OverlappedComponent :type "PrimitiveComponent Object Reference") (OtherActor :type "Actor Object Reference") (OtherComp :type "PrimitiveComponent Object Reference") (OtherBodyIndex :type Integer) (bFromSweep :type Boolean) (SweepResult :type "HitResult Structure (by ref)"))
  (`/Engine/EditorBlueprintResources/ActorMacros.Switch Has Authority`
    (:`Authority`
      (message `/Game/Blueprints/BlueprintInterface/BPI_HandleDamage.Damaged` OtherActor (`self.AttackPower`) null))))

(fn `UserConstructionScript`)