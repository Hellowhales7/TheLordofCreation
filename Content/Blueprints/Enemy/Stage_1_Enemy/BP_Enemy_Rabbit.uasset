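; BP_Enemy_Rabbit is a Stage 1 rabbit enemy that builds on parent class behavior.
; On BeginPlay it runs server init, sets its combat, movement and EXP drop attributes, and starts a looping timer that calls FindNearestPlayer.
; On death it plays the rabbit death animation, sets the Death flag and destroys itself after a short delay.
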(event `self.ReceiveBeginPlay`
  (`parent.ReceiveBeginPlay`)
  (`self.Server_Init`)
  (`self.SetAttributes` 100.0 100.0 10 0.0 20.0 300.0)
  (`KismetSystemLibrary.K2_SetTimer` null "FindNearestPlayer" 0.5 true))

(event `self.ReceiveTick`
  (params (DeltaSeconds :type "Float (single-precision)"))
  (`parent.ReceiveTick` DeltaSeconds))

(event `self.Die`
  (`parent.Die`)
  (`SkeletalMeshComponent.PlayAnimation` (`self.Mesh`) "/Game/Fab/ForestAnimalsPack/Rabbit/Animations/ANIM_Rabbit_Death.ANIM_Rabbit_Death" false)
  (set `self.Death` true)
  (`KismetSystemLibrary.Delay` 1.5)
  (`self.K2_DestroyActor`))

(fn `UserConstructionScript`
  (`parent.UserConstructionScript`))