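; Base enemy that chases players, damages them on contact and drops BP_Exp when it dies.
; BeginPlay applies GAS initial attributes, fills the health bar and starts a timer steering the AI controller toward the nearer of the first two characters.
; Capsule overlap starts repeated contact checks; end overlap resets them to one last check.
; Contact kills the enemy if the player is invincible, otherwise damages the player and grants invincibility.
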(event `self.ReceiveBeginPlay`
  (bind _asbp_enemy_aicontroller (cast `/Game/Blueprints/Enemy/BP_EnemyAIController` (`AIBlueprintHelperLibrary.GetAIController` self)))
  (set `self.BP Enemy AIController` _asbp_enemy_aicontroller)
  (bind _aswbp_enemy_health_bar (cast `/Game/Blueprints/Enemy/EnemyUI/WBP_EnemyHealthBar` (`WidgetComponent.GetUserWidgetObject` (`self.HpBar`))))
  (bind _output_get (set `self.Health UI` _aswbp_enemy_health_bar))
  (`Widget.SetVisibility` _output_get "Visible")
  (`AbilitySystemComponent.BP_ApplyGameplayEffectToSelf` :`self` (`self.AbilitySystemComponent`) :`GameplayEffectClass` "/Game/Blueprints/GAS/GE/GE_InitEnemyAtributes.GE_InitEnemyAtributes_C")
  (`self.SetHealthPercent`)
  (`KismetSystemLibrary.K2_SetTimer` null "FindNearestPlayer" 0.5 true))

(event `self.ReceiveTick`
  (params (DeltaSeconds :type "Float (single-precision)")))

(event `self.CapsuleComponent.OnComponentBeginOverlap`
  (params (OverlappedComponent :type "PrimitiveComponent Object Reference") (OtherActor :type "Actor Object Reference") (OtherComp :type "PrimitiveComponent Object Reference") (OtherBodyIndex :type Integer) (bFromSweep :type Boolean) (SweepResult :type "HitResult Structure (by ref)"))
  (cast `/Game/Blueprints/Character/BP_MSCharacter` OtherActor)
  (`KismetSystemLibrary.K2_SetTimer` null "CheckingOverlap" 0.2 true))

(event `self.CapsuleComponent.OnComponentEndOverlap`
  (params (OverlappedComponent :type "PrimitiveComponent Object Reference") (OtherActor :type "Actor Object Reference") (OtherComp :type "PrimitiveComponent Object Reference") (OtherBodyIndex :type Integer))
  (cast `/Game/Blueprints/Character/BP_MSCharacter` OtherActor)
  (`KismetSystemLibrary.K2_SetTimer` null "CheckingOverlap" 0.2))

(event `Die`
  (`KismetSystemLibrary.PrintString` "EnemyDie")
  (`|SpawnActorFromClass` "/Game/Blueprints/Enemy/BP_Exp.BP_Exp_C" (`self.GetTransform`) "Undefined" "MultiplyWithRoot" null null)
  (`KismetSystemLibrary.Delay` 0.2)
  (`self.K2_DestroyActor`))

(fn `CheckingOverlap`
  (for _array_element (`PrimitiveComponent.GetOverlappingActors` (`self.CapsuleComponent`) "/Game/Blueprints/Character/BP_MSCharacter.BP_MSCharacter_C")
    (bind _asbp_mscharacter (cast `/Game/Blueprints/Character/BP_MSCharacter` _array_element))
    (if (`/Game/Blueprints/Character/BP_MSCharacter.bInvincible` _asbp_mscharacter)
      (`self.Die`)
      (else
        (message `/Game/Blueprints/BPI_HandleDamage.Damaged` _asbp_mscharacter)
        (`/Game/Blueprints/Character/BP_MSCharacter.Apply Invincible` _asbp_mscharacter)))))

(fn `FindNearestPlayer`
  (locals (Distances :type "Array of Float (double-precision)") (Characters :type "Array of /Game/Blueprints/Character/BP_MSCharacter Object Reference"))
  (bind _distances (`local.Distances`))
  (bind _bp_enemy_aicontroller (`self.BP Enemy AIController`))
  (bind _bp_enemy_aicontroller_2 (`self.BP Enemy AIController`))
  (bind _outactors (`GameplayStatics.GetAllActorsOfClass` "/Game/Blueprints/Character/BP_MSCharacter.BP_MSCharacter_C"))
  (bind _output_get (set `local.Characters` _outactors))
  (for (_array_element _array_index) _output_get
    (`KismetArrayLibrary.Array_Set` (`local.Distances`) _array_index (`KismetMathLibrary.Vector_Distance` (`self.K2_GetActorLocation` _array_element) (`self.K2_GetActorLocation`)) true))
  (if (< (`|GetArrayItem` _distances) (`|GetArrayItem` _distances 1))
    (`/Engine/EditorBlueprintResources/StandardMacros.IsValid` _bp_enemy_aicontroller
      (:`Is Valid`
        (`AIController.MoveToActor` _bp_enemy_aicontroller (`|GetArrayItem` (`local.Characters`)) 1.0 true true true null true)))
    (else
      (`/Engine/EditorBlueprintResources/StandardMacros.IsValid` _bp_enemy_aicontroller_2
        (:`Is Valid`
          (`AIController.MoveToActor` _bp_enemy_aicontroller_2 (`|GetArrayItem` (`local.Characters`) 1) 1.0 true true true null true))))))

(fn `Initalize`
  (`AbilitySystemComponent.BP_ApplyGameplayEffectToSelf` :`self` (`self.AbilitySystemComponent`) :`GameplayEffectClass` "/Game/Blueprints/GAS/GE/GE_InitEnemyAtributes.GE_InitEnemyAtributes_C")
  (bind _aswbp_enemy_health_bar (cast `/Game/Blueprints/Enemy/EnemyUI/WBP_EnemyHealthBar` (`WidgetComponent.GetUserWidgetObject` (`self.HpBar`))))
  (bind _output_get (set `self.Health UI` _aswbp_enemy_health_bar))
  (`Widget.SetVisibility` _output_get "Visible"))

(fn `SetHealthPercent`
  (bind _playerattributeset (`self.PlayerAttributeSet`))
  (bind (_maxhealth_basevalue _maxhealth_currentvalue) (break `GameplayAttributeData` (`PlayerAttributeSet.MaxHealth` _playerattributeset)))
  (bind (_health_basevalue _health_currentvalue) (break `GameplayAttributeData` (`PlayerAttributeSet.Health` _playerattributeset)))
  (set `/Game/Blueprints/Enemy/EnemyUI/WBP_EnemyHealthBar.HealthPercent` (/ _health_currentvalue _maxhealth_currentvalue) (`self.Health UI`)))

(fn `UserConstructionScript`)