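; GA_HealthRegen is a Gameplay Ability that, despite its name, holds Cloth augmentation barrier logic.
; On server activation it commits, applies GE_CoolDown_Cloth with a SetByCaller magnitude from BaseCDT, then only casts the owner.
; ChargeCloth sets the character's Barrier by ability level, first calling CreateCloth to spawn and attach BP_Cloth if Barrier is zero.
; Nothing here calls ChargeCloth, and the HealthRegen attribute read is unused.
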(event `self.K2_ActivateAbility`
  (`self.K2_HasAuthority`
    (:`True`
      (`self.K2_CommitAbility`)
      (bind _returnvalue (`AbilitySystemBlueprintLibrary.AssignTagSetByCallerMagnitude` (`self.MakeOutgoingGameplayEffectSpec` "/Game/Blueprints/GAS/GE/GE_CoolDown_Cloth.GE_CoolDown_Cloth_C") (struct :`TagName` "Ability.Augmentation.Cloth") (`self.BaseCDT`)))
      (`self.K2_ApplyGameplayEffectSpecToOwner` _returnvalue)
      (bind _asbp_mscharacter (cast `/Game/Blueprints/Character/BP_MSCharacter` (`self.GetOwningActorFromActorInfo`))))))

(fn `ChargeCloth`
  (bind _asbp_mscharacter (cast `/Game/Blueprints/Character/BP_MSCharacter` (`self.GetOwningActorFromActorInfo`)))
  (if (== (`/Game/Blueprints/Character/BP_MSCharacter.Barrier` _asbp_mscharacter) 0)
    (`self.CreateCloth`))
  (switch `int` (`self.GetAbilityLevel`)
    (:`Default`
      (set `/Game/Blueprints/Character/BP_MSCharacter.Barrier` 1 _asbp_mscharacter :!label _label))
    (:`0`
      (goto _label))
    (:`1`
      (goto _label))
    (:`2`
      (set `/Game/Blueprints/Character/BP_MSCharacter.Barrier` 2 _asbp_mscharacter :!label _label_2))
    (:`3`
      (goto _label_2))
    (:`4`
      (goto _label_2))
    (:`5`
      (set `/Game/Blueprints/Character/BP_MSCharacter.Barrier` 3 _asbp_mscharacter))))

(fn `CreateCloth`
  (bind _returnvalue (`self.GetOwningActorFromActorInfo`))
  (bind _returnvalue_2 (`|SpawnActorFromClass` "/Game/Blueprints/GAS/GA/Augmentation/Object/BP_Cloth.BP_Cloth_C" (`Actor.GetTransform` _returnvalue) "Undefined" "MultiplyWithRoot" null 0 null))
  (`Actor.K2_AttachToActor` _returnvalue_2 _returnvalue "None" "KeepWorld" "KeepWorld" "KeepWorld" true))