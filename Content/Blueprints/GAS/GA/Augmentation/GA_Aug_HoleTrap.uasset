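; Gameplay ability for the Hole Trap augmentation that places a BP_Hole actor slightly below the owner's position.
; On activation, only with authority, it commits, applies GE_CoolDown_HoleTrap with a set-by-caller magnitude from CDT, spawns the hole and ends.
; A ThrowRock function spawns BP_Rock at a yaw offset from the owner's forward vector, but nothing in this file calls it.
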(event `self.K2_ActivateAbility`
  (bind _returnvalue (`Actor.GetTransform` (`self.GetOwningActorFromActorInfo`)))
  (`self.K2_HasAuthority`
    (:`True`
      (`self.K2_CommitAbility`)
      (bind _returnvalue_2 (`AbilitySystemBlueprintLibrary.AssignTagSetByCallerMagnitude` (`self.MakeOutgoingGameplayEffectSpec` "/Game/Blueprints/GAS/GE/GE_CoolDown_HoleTrap.GE_CoolDown_HoleTrap_C") (struct :`TagName` "Ability.Augmentation.Hole") (`self.CDT`)))
      (`self.K2_ApplyGameplayEffectSpecToOwner` _returnvalue_2)
      (`|SpawnActorFromClass` "/Game/Blueprints/GAS/GA/Augmentation/BP_Hole.BP_Hole_C" (`KismetMathLibrary.MakeTransform` (`KismetMathLibrary.MakeVector` (.x (.location _returnvalue)) (.y (.location _returnvalue)) (- (.z (.location _returnvalue)) 40.0)) (.rotation _returnvalue) (.scale _returnvalue)) "Undefined" "MultiplyWithRoot" null null)
      (`self.K2_EndAbility`))))

(fn `Throw Rock`
  (params (direction :type "Float (double-precision)"))
  (bind _returnvalue (`self.GetOwningActorFromActorInfo`))
  (bind (_returnvalue_roll _returnvalue_pitch _returnvalue_yaw) (`KismetMathLibrary.BreakRotator` (`Actor.K2_GetActorRotation` (`Actor.Instigator` _returnvalue))))
  (`|SpawnActorFromClass` "/Game/Blueprints/GAS/GA/Augmentation/BP_Rock.BP_Rock_C" (`KismetMathLibrary.MakeTransform` (+ (`Actor.K2_GetActorLocation` _returnvalue) (0.0 0.0 0.0) (`KismetMathLibrary.GreaterGreater_VectorRotator` (* (`Actor.GetActorForwardVector` _returnvalue) (50.0 50.0 50.0)) (`KismetMathLibrary.MakeRotator` 0.0 0.0 direction))) (`KismetMathLibrary.MakeRotator` _returnvalue_roll _returnvalue_pitch (+ _returnvalue_yaw direction))) "Undefined" "MultiplyWithRoot" null null))