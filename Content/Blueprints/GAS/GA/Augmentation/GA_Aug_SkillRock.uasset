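; Gameplay ability for the Rock augmentation skill, throwing a fan of BP_Rock projectiles from the owning actor.
; On authority, it commits and applies GE_CoolDown_Rock with a SetByCaller duration.
; Ability level sets the rock count, up to five, adding alternating yaw offsets around the forward direction.
; ThrowRock spawns each rock ahead of and below the owner's location, passing the parent class's attack calculation.
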(event `self.K2_ActivateAbility`
  (`self.K2_HasAuthority`
    (:`True`
      (`self.K2_CommitAbility`)
      (bind _returnvalue (`AbilitySystemBlueprintLibrary.AssignTagSetByCallerMagnitude` (`self.MakeOutgoingGameplayEffectSpec` "/Game/Blueprints/GAS/GE/GE_CoolDown_Rock.GE_CoolDown_Rock_C") (struct :`TagName` "Ability.Augmentation.Rock") (`self.CDT`)))
      (`self.K2_ApplyGameplayEffectSpecToOwner` _returnvalue)
      (switch `int` (`self.GetAbilityLevel`)
        (:`Default`
          (`self.Throw Rock` 0.0 :!label _label)
          (`self.K2_EndAbility`))
        (:`0`
          (goto _label))
        (:`1`
          (goto _label))
        (:`2`
          (`self.Throw Rock` 0.0)
          (`self.Throw Rock` -15.0)
          (`self.K2_EndAbility`))
        (:`3`
          (`self.Throw Rock` 0.0)
          (`self.Throw Rock` -15.0)
          (`self.Throw Rock` 15.0)
          (`self.K2_EndAbility`))
        (:`4`
          (`self.Throw Rock` 0.0)
          (`self.Throw Rock` -15.0)
          (`self.Throw Rock` 15.0)
          (`self.Throw Rock` -30.0)
          (`self.K2_EndAbility`))
        (:`5`
          (`self.Throw Rock` 0.0)
          (`self.Throw Rock` -15.0)
          (`self.Throw Rock` 15.0)
          (`self.Throw Rock` -30.0)
          (`self.Throw Rock` 30.0)
          (`self.K2_EndAbility`))))))

(fn `CalculateAttack`
  (returns (OutAttack :type "Float (double-precision)"))
  (return (`parent.CalculateAttack`)))

(fn `Throw Rock`
  (params (direction :type "Float (double-precision)"))
  (bind _returnvalue (`self.GetOwningActorFromActorInfo`))
  (bind (_returnvalue_roll _returnvalue_pitch _returnvalue_yaw) (`KismetMathLibrary.BreakRotator` (`Actor.K2_GetActorRotation` (`Actor.Instigator` _returnvalue))))
  (`|SpawnActorFromClass` "/Game/Blueprints/GAS/GA/Augmentation/Object/BP_Rock.BP_Rock_C" (`KismetMathLibrary.MakeTransform` (+ (`Actor.K2_GetActorLocation` _returnvalue) (0.0 0.0 -50.0) (`KismetMathLibrary.GreaterGreater_VectorRotator` (* (`Actor.GetActorForwardVector` _returnvalue) (50.0 50.0 50.0)) (`KismetMathLibrary.MakeRotator` 0.0 0.0 direction))) (`KismetMathLibrary.MakeRotator` _returnvalue_roll _returnvalue_pitch (+ _returnvalue_yaw direction))) "Undefined" "MultiplyWithRoot" null (`self.CalculateAttack`) null))