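; BP_Club is a spiked club actor from the GAS augmentation set that makes one swing, damaging what it hits.
; Tick eases its relative yaw slightly past TargetRotate, destroying the actor once that angle is reached.
; On overlap, the authority records each new actor in AffectedEnemy so it is hit once, prints its name, and applies Attack damage through ServerApplyDamage on the BP_MSCharacter that GetActorOfClass found at BeginPlay.
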(event `self.ReceiveBeginPlay`
  (bind _returnvalue (`GameplayStatics.GetActorOfClass` "/Game/Blueprints/Character/BP_MSCharacter.BP_MSCharacter_C"))
  (set `self.BP MSCharacter` _returnvalue))

(event `self.ReceiveTick`
  (params (DeltaSeconds :type "Float (single-precision)"))
  (`self.K2_SetActorRelativeRotation` (`KismetMathLibrary.MakeRotator` 0.0 0.0 (`KismetMathLibrary.FInterpTo` (`KismetMathLibrary.ClampAxis` (.yaw (.rotation (`SceneComponent.GetRelativeTransform` (`self.Scene`))))) (+ (`self.TargetRotate`) 5.0) DeltaSeconds 10.0)))
  (if (>= (`KismetMathLibrary.ClampAxis` (.yaw (.rotation (`SceneComponent.GetRelativeTransform` (`self.Scene`))))) (`self.TargetRotate`))
    (`self.K2_DestroyActor`)))

(event `self.spiked_club.OnComponentBeginOverlap`
  (params (OverlappedComponent :type "PrimitiveComponent Object Reference") (OtherActor :type "Actor Object Reference") (OtherComp :type "PrimitiveComponent Object Reference") (OtherBodyIndex :type Integer) (bFromSweep :type Boolean) (SweepResult :type "HitResult Structure (by ref)"))
  (if (== (`KismetArrayLibrary.Array_Find` (`self.AffectedEnemy`) OtherActor) -1)
    (`/Engine/EditorBlueprintResources/ActorMacros.Switch Has Authority`
      (:`Authority`
        (`KismetSystemLibrary.PrintString` (`KismetSystemLibrary.GetDisplayName` OtherActor))
        (`KismetArrayLibrary.Array_Add` (`self.AffectedEnemy`) OtherActor)
        (`/Game/Blueprints/Character/BP_MSCharacter.Server_ApplyDamage` (`self.BP MSCharacter`) OtherActor (`self.Attack`))))))

(fn `UserConstructionScript`)