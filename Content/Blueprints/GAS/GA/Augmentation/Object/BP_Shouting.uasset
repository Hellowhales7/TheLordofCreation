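; BP_Shouting is an augmentation actor that acts as an expanding shout, slowing actors its sphere touches.
; Tick grows its scale toward Scope0 at constant speed and destroys it once X reaches base size times Scope0.
; On authority, each newly overlapped actor is recorded in AffectedEnemy and sent a slowdown multiplier derived from SlowPer.
; It also applies zero damage to that actor through the first BP_MSCharacter found at BeginPlay.
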(event `self.ReceiveBeginPlay`
  (bind _returnvalue (`GameplayStatics.GetActorOfClass` "/Game/Blueprints/Character/BP_MSCharacter.BP_MSCharacter_C"))
  (set `self.BP MSCharacter` _returnvalue))

(event `self.ReceiveTick`
  (params (DeltaSeconds :type "Float (single-precision)"))
  (bind _returnvalue_x (`KismetMathLibrary.BreakVector` (`self.GetActorScale3D`)))
  (bind _basesize_x (`KismetMathLibrary.BreakVector` (`self.BaseSize`)))
  (`self.SetActorScale3D` (`KismetMathLibrary.VInterpTo_Constant` (`self.GetActorScale3D` self) (`KismetMathLibrary.Conv_DoubleToVector` (`self.Scope_0`)) DeltaSeconds 6.0))
  (if (>= _returnvalue_x (* _basesize_x (`self.Scope_0`)))
    (`self.K2_DestroyActor`)))

(event `self.Sphere.OnComponentBeginOverlap`
  (params (OverlappedComponent :type "PrimitiveComponent Object Reference") (OtherActor :type "Actor Object Reference") (OtherComp :type "PrimitiveComponent Object Reference") (OtherBodyIndex :type Integer) (bFromSweep :type Boolean) (SweepResult :type "HitResult Structure (by ref)"))
  (bind _slowper (`self.SlowPer`))
  (if (== (`KismetArrayLibrary.Array_Find` (`self.AffectedEnemy`) OtherActor) -1)
    (`/Engine/EditorBlueprintResources/ActorMacros.Switch Has Authority`
      (:`Authority`
        (`KismetArrayLibrary.Array_Add` (`self.AffectedEnemy`) OtherActor)
        (`KismetSystemLibrary.PrintString` (`KismetStringLibrary.Conv_DoubleToString` _slowper) true true (struct :`R` 1.0 :`G` 0.518708 :`A` 1.0) 2.0 "1")
        (message `/Game/Blueprints/BlueprintInterface/BPI_HandleSlowdown.Slowdown` OtherActor (- 1.0 (/ _slowper 100.0)))
        (`/Game/Blueprints/Character/BP_MSCharacter.Server_ApplyDamage` (`self.BP MSCharacter`) OtherActor 0.0)))))

(fn `UserConstructionScript`)