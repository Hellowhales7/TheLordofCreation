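; BP_Shouting is a short-lived area-damage actor, apparently for the Shouting augmentation ability, that acts as an expanding burst.
; Tick grows the actor toward triple scale at constant speed and destroys it after half a second.
; Sphere overlaps on the authority apply fixed damage through ServerApplyDamage on the first BP_MSCharacter found at BeginPlay, with no target filtering.
; A SlowdownMessage call is left unconnected.
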(event `self.ReceiveBeginPlay`
  (bind _returnvalue (`GameplayStatics.GetActorOfClass` "/Game/Blueprints/Character/BP_MSCharacter.BP_MSCharacter_C"))
  (set `self.BP MSCharacter` _returnvalue))

(event `self.ReceiveTick`
  (params (DeltaSeconds :type "Float (single-precision)"))
  (bind _output_get (set `self.Timer` (+ (`self.Timer`) DeltaSeconds)))
  (if (> _output_get 0.5)
    (`self.K2_DestroyActor`)
    (else
      (`self.SetActorScale3D` (`KismetMathLibrary.VInterpTo_Constant` (`self.GetActorScale3D` self) (3.0 3.0 3.0) DeltaSeconds 6.0)))))

(event `self.Sphere.OnComponentBeginOverlap`
  (params (OverlappedComponent :type "PrimitiveComponent Object Reference") (OtherActor :type "Actor Object Reference") (OtherComp :type "PrimitiveComponent Object Reference") (OtherBodyIndex :type Integer) (bFromSweep :type Boolean) (SweepResult :type "HitResult Structure (by ref)"))
  (`/Engine/EditorBlueprintResources/ActorMacros.Switch Has Authority`
    (:`Authority`
      (`/Game/Blueprints/Character/BP_MSCharacter.Server_ApplyDamage` (`self.BP MSCharacter`) OtherActor 10.0))))

(fn `UserConstructionScript`)