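; Gameplay ability for the Club augmentation, which spawns a BP_Club attached to the owner.
; On the authority, it commits, applies GE_CoolDown_Club with a calculated cooldown passed by SetByCaller tag, then ends right after spawning.
; Ability level selects the club's target rotation, widening from a quarter turn to nearly a full circle.
; The club's attack value comes from the parent class's CalculateAttack.
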(event `self.K2_ActivateAbility`
  (`self.K2_HasAuthority`
    (:`True`
      (`self.K2_CommitAbility`)
      (bind _returnvalue (`AbilitySystemBlueprintLibrary.AssignTagSetByCallerMagnitude` (`self.MakeOutgoingGameplayEffectSpec` "/Game/Blueprints/GAS/GE/GE_CoolDown_Club.GE_CoolDown_Club_C") (struct :`TagName` "Ability.Augmentation.Club") (`self.CalculateCDT`)))
      (`self.K2_ApplyGameplayEffectSpecToOwner` _returnvalue)
      (switch `int` (`self.GetAbilityLevel`)
        (:`0`
          (`self.CreateClub` 90.0 :!label _label)
          (`self.K2_EndAbility`))
        (:`1`
          (goto _label))
        (:`2`
          (`self.CreateClub` 90.0)
          (`self.K2_EndAbility`))
        (:`3`
          (`self.CreateClub` 180.0 :!label _label_2)
          (`self.K2_EndAbility`))
        (:`4`
          (goto _label_2))
        (:`5`
          (`self.CreateClub` 354.0)
          (`self.K2_EndAbility`))))))

(fn `CalculateAttack`
  (returns (OutAttack :type "Float (double-precision)"))
  (return (`parent.CalculateAttack`)))

(fn `CreateClub`
  (params (TargetRotation :type "Float (double-precision)"))
  (bind _returnvalue (`self.GetOwningActorFromActorInfo`))
  (bind (_returnvalue_location _returnvalue_rotation _returnvalue_scale) (`KismetMathLibrary.BreakTransform` (`Actor.GetTransform` _returnvalue)))
  (bind _returnvalue_2 (`|SpawnActorFromClass` "/Game/Blueprints/GAS/GA/Augmentation/Object/BP_Club.BP_Club_C" (`KismetMathLibrary.MakeTransform` _returnvalue_location (struct) _returnvalue_scale) "Undefined" "MultiplyWithRoot" null TargetRotation (`self.CalculateAttack`) null))
  (`Actor.K2_AttachToActor` _returnvalue_2 _returnvalue "None" "KeepWorld" "KeepRelative" "KeepWorld" true))