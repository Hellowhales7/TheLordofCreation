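; Gameplay ability for the Shouting augmentation, which spawns a shout actor on its owner with a configurable scope and slow.
; On server activation it commits, applies the Shouting cooldown effect with BaseCDT as a SetByCaller magnitude, calls CreateShouting, then ends.
; CreateShouting spawns BP_Shouting at the owner, passing in calculated scope and slow percentage, and attaches it to the owner.
; A ThrowRock function that spawns BP_Rock is present but never called here.
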(event `self.K2_ActivateAbility`
  (`self.K2_HasAuthority`
    (:`True`
      (`self.K2_CommitAbility`)
      (bind _returnvalue (`AbilitySystemBlueprintLibrary.AssignTagSetByCallerMagnitude` (`self.MakeOutgoingGameplayEffectSpec` "/Game/Blueprints/GAS/GE/GE_CoolDown_Shouting.GE_CoolDown_Shouting_C") (struct :`TagName` "Ability.Augmentation.Shouting") (`self.BaseCDT`)))
      (`self.K2_ApplyGameplayEffectSpecToOwner` _returnvalue)
      (`self.CreateShouting`)
      (`self.K2_EndAbility`))))

(fn `CreateShouting`
  (bind _returnvalue (`self.GetOwningActorFromActorInfo`))
  (bind (_returnvalue_roll _returnvalue_pitch _returnvalue_yaw) (`KismetMathLibrary.BreakRotator` (`Actor.K2_GetActorRotation` (`Actor.Instigator` _returnvalue))))
  (bind _returnvalue_2 (`|SpawnActorFromClass` "/Game/Blueprints/GAS/GA/Augmentation/Object/BP_Shouting.BP_Shouting_C" (`KismetMathLibrary.MakeTransform` (+ (`Actor.K2_GetActorLocation` _returnvalue) (0.0 0.0 0.0) (`KismetMathLibrary.GreaterGreater_VectorRotator` (* (`Actor.GetActorForwardVector` _returnvalue) (0.0 0.0 0.0)) (`KismetMathLibrary.MakeRotator` 0.0))) (`KismetMathLibrary.MakeRotator` _returnvalue_roll _returnvalue_pitch (+ _returnvalue_yaw 0.0))) "Undefined" "MultiplyWithRoot" null (`self.CalculateScope`) (`self.CalculateSlowPer`) null))
  (`Actor.K2_AttachToActor` _returnvalue_2 _returnvalue "None" "KeepWorld" "KeepWorld" "KeepWorld" true))

(fn `Throw Rock`
  (params (direction :type "Float (double-precision)"))
  (bind _returnvalue (`self.GetOwningActorFromActorInfo`))
  (bind (_returnvalue_roll _returnvalue_pitch _returnvalue_yaw) (`KismetMathLibrary.BreakRotator` (`Actor.K2_GetActorRotation` (`Actor.Instigator` _returnvalue))))
  (`|SpawnActorFromClass` "/Game/Blueprints/GAS/GA/Augmentation/Object/BP_Rock.BP_Rock_C" (`KismetMathLibrary.MakeTransform` (+ (`Actor.K2_GetActorLocation` _returnvalue) (0.0 0.0 0.0) (`KismetMathLibrary.GreaterGreater_VectorRotator` (* (`Actor.GetActorForwardVector` _returnvalue) (50.0 50.0 50.0)) (`KismetMathLibrary.MakeRotator` 0.0 0.0 direction))) (`KismetMathLibrary.MakeRotator` _returnvalue_roll _returnvalue_pitch (+ _returnvalue_yaw direction))) "Undefined" "MultiplyWithRoot" null 10.0 null))