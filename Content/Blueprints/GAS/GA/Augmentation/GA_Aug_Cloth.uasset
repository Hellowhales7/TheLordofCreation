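; Gameplay ability for the Cloth augmentation that grants the player a single Barrier charge with an attached BP_Cloth actor.
; On activation it commits and applies the Cloth cooldown effect, setting its magnitude by caller tag from CDT.
; If the player character's Barrier is below one, it increments it and attaches the spawned cloth, then ends.
; A ThrowRock function spawns BP_Rock at a yaw offset but is not called here.
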(event `self.K2_ActivateAbility`
  (bind _returnvalue (`GameplayStatics.GetPlayerCharacter` 0))
  (`self.K2_CommitAbility`)
  (bind _returnvalue_2 (`AbilitySystemBlueprintLibrary.AssignTagSetByCallerMagnitude` (`self.MakeOutgoingGameplayEffectSpec` "/Game/Blueprints/GAS/GE/GE_CoolDown_Cloth.GE_CoolDown_Cloth_C") (struct :`TagName` "Ability.Augmentation.Cloth") (`self.CDT`)))
  (`self.K2_ApplyGameplayEffectSpecToOwner` _returnvalue_2)
  (bind _asbp_mscharacter (cast `/Game/Blueprints/Character/BP_MSCharacter` _returnvalue))
  (bind _barrier (`/Game/Blueprints/Character/BP_MSCharacter.Barrier` _asbp_mscharacter))
  (if (< _barrier 1)
    (bind _result (`/Engine/EditorBlueprintResources/StandardMacros.IncrementInt` _barrier)
      (:`  `
        (set `/Game/Blueprints/Character/BP_MSCharacter.Barrier` _result _asbp_mscharacter)
        (bind _returnvalue_3 (`|SpawnActorFromClass` "/Game/Blueprints/GAS/GA/Augmentation/BP_Cloth.BP_Cloth_C" (`Actor.GetTransform` _returnvalue) "Undefined" "MultiplyWithRoot" null null))
        (`Actor.K2_AttachToActor` _returnvalue_3 _returnvalue "None" "KeepWorld" "KeepWorld" "KeepWorld" true))))
  (`self.K2_EndAbility`))

(fn `Throw Rock`
  (params (direction :type "Float (double-precision)"))
  (bind _returnvalue (`self.GetOwningActorFromActorInfo`))
  (bind (_returnvalue_roll _returnvalue_pitch _returnvalue_yaw) (`KismetMathLibrary.BreakRotator` (`Actor.K2_GetActorRotation` (`Actor.Instigator` _returnvalue))))
  (`|SpawnActorFromClass` "/Game/Blueprints/GAS/GA/Augmentation/BP_Rock.BP_Rock_C" (`KismetMathLibrary.MakeTransform` (+ (`Actor.K2_GetActorLocation` _returnvalue) (0.0 0.0 0.0) (`KismetMathLibrary.GreaterGreater_VectorRotator` (* (`Actor.GetActorForwardVector` _returnvalue) (50.0 50.0 50.0)) (`KismetMathLibrary.MakeRotator` 0.0 0.0 direction))) (`KismetMathLibrary.MakeRotator` _returnvalue_roll _returnvalue_pitch (+ _returnvalue_yaw direction))) "Undefined" "MultiplyWithRoot" null null))