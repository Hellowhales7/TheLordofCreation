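; BP_Rock is a physics-driven rock projectile that deals damage to actors it overlaps.
; On BeginPlay it launches Rock0 along its forward vector with a mass-independent, mostly horizontal impulse and caches the first BP_MSCharacter found in the world.
; Sphere overlaps, on authority only, route fixed damage through that character's ServerApplyDamage, with no target filtering.
; A Tick timer destroys the rock after two seconds.
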(event `self.ReceiveBeginPlay`
  (bind _returnvalue (`GameplayStatics.GetActorOfClass` "/Game/Blueprints/Character/BP_MSCharacter.BP_MSCharacter_C"))
  (set `self.BP MSCharacter` _returnvalue)
  (`PrimitiveComponent.AddImpulse` (`self.Rock_0`) (* (`self.GetActorForwardVector`) (2500.0 2500.0 1.0)) "None" true))

(event `self.ReceiveActorBeginOverlap`
  (params (OtherActor :type "Actor Object Reference")))

(event `self.ReceiveTick`
  (params (DeltaSeconds :type "Float (single-precision)"))
  (bind _output_get (set `self.timer` (+ DeltaSeconds (`self.timer`))))
  (if (>= _output_get 2.0)
    (`self.K2_DestroyActor`)))

(event `self.Sphere.OnComponentBeginOverlap`
  (params (OverlappedComponent :type "PrimitiveComponent Object Reference") (OtherActor :type "Actor Object Reference") (OtherComp :type "PrimitiveComponent Object Reference") (OtherBodyIndex :type Integer) (bFromSweep :type Boolean) (SweepResult :type "HitResult Structure (by ref)"))
  (`/Engine/EditorBlueprintResources/ActorMacros.Switch Has Authority`
    (:`Authority`
      (`/Game/Blueprints/Character/BP_MSCharacter.Server_ApplyDamage` (`self.BP MSCharacter`) OtherActor 10.0))))

(fn `UserConstructionScript`)