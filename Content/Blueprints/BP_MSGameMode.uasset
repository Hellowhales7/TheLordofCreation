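; BP_MSGameMode is a game mode that tracks player deaths and triggers game over when every BP_MSCharacter is down.
; PlayerDeathAlert increments DeathCount and compares it to the number of BP_MSCharacter actors currently in the world, calling GameOver when they match.
; PlayerReviveAlert decrements the count, while GameOver sets the GameOver flag on every character.
; GameOver and revive events also print debug strings.
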(event `self.ReceiveBeginPlay`)

(event `self.ReceiveTick`
  (params (DeltaSeconds :type "Float (single-precision)")))

(event `GameOver`
  (bind _outactors (`GameplayStatics.GetAllActorsOfClass` "/Game/Blueprints/Character/BP_MSCharacter.BP_MSCharacter_C"))
  (for _array_element _outactors
    (set `/Game/Blueprints/Character/BP_MSCharacter.GameOver` true _array_element))
  (`KismetSystemLibrary.PrintString` (`KismetTextLibrary.Conv_TextToString` (`|FormatText` "death count {int} game over" (`self.DeathCount`)))))

(event `PlayerDeathAlert`
  (bind _outactors (`GameplayStatics.GetAllActorsOfClass` "/Game/Blueprints/Character/BP_MSCharacter.BP_MSCharacter_C"))
  (set `self.PlayerAmount` (`KismetArrayLibrary.Array_Length` _outactors))
  (`/Engine/EditorBlueprintResources/StandardMacros.IncrementInt` (`self.DeathCount`)
    (:`  `
      (if (== (`self.DeathCount`) (`self.PlayerAmount`))
        (`self.GameOver`)))))

(event `PlayerReviveAlert`
  (`/Engine/EditorBlueprintResources/StandardMacros.DecrementInt` (`self.DeathCount`)
    (:`  `
      (`KismetSystemLibrary.PrintString` "revive")
      (`KismetSystemLibrary.PrintString` (`KismetTextLibrary.Conv_TextToString` (`|FormatText` "death count {int} " (`self.DeathCount`)))))))

(fn `UserConstructionScript`)